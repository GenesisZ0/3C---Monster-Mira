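; Door actor that swings by yaw, apparently driven by mouse movement, through a custom event taking a turn rate and sensitivity.
; The event rotates the door mesh locally and sets TED on the first-person character cached at BeginPlay.
; Tick zeroes TurnRate and prints the yaw when mouse X and the player are both still.
; OpenDoor is empty, the reverse-rotation branch never runs, and the stored MinAngle is unused.
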(event `self.ReceiveTick`
  (params (DeltaSeconds :type "Float (single-precision)"))
  (bind (_returnvalue_roll _returnvalue_pitch _returnvalue_yaw) (`KismetMathLibrary.BreakRotator` (`SceneComponent.K2_GetComponentRotation` (`self.door1_door`))))
  (if (!= (`PlayerController.GetInputMouseDelta` (`GameplayStatics.GetPlayerController` 0)) 0.0)
    _
    (elif (`/Game/FirstPerson/Blueprints/BP_FirstPersonCharacter.NotMooving` (`self.PlayerRef`))
      (set `self.TurnRate` 0.0)
      (`KismetSystemLibrary.PrintString` (`KismetStringLibrary.Conv_DoubleToString` _returnvalue_yaw)))))

(event `CustomEvent`
  (params (TurnRate :type "Float (double-precision)") (Sensi :type "Float (double-precision)"))
  (bind (_returnvalue_roll _returnvalue_pitch _returnvalue_yaw) (`KismetMathLibrary.BreakRotator` (`KismetMathLibrary.MakeRotator` 0.0 0.0 (* (`self.TurnRate`) Sensi))))
  (if true
    (`SceneComponent.K2_AddLocalRotation` (`self.door1_door`) (`KismetMathLibrary.MakeRotator` 0.0 0.0 _returnvalue_yaw) false false)
    (set `/Game/FirstPerson/Blueprints/BP_FirstPersonCharacter.TED` true (`self.PlayerRef`))))

(event `self.ReceiveBeginPlay`
  (bind (_returnvalue_roll _returnvalue_pitch _returnvalue_yaw) (`KismetMathLibrary.BreakRotator` (`SceneComponent.K2_GetComponentRotation` (`self.door1_door`))))
  (set `self.MinAngle` _returnvalue_yaw)
  (bind _returnvalue (`GameplayStatics.GetActorOfClass` "/Game/FirstPerson/Blueprints/BP_FirstPersonCharacter.BP_FirstPersonCharacter_C"))
  (set `self.PlayerRef` _returnvalue))

(event `OpenDoor`)

(fn `UserConstructionScript`)